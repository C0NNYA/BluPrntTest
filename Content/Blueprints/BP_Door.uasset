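; BP_Door is an interactable swinging door that shows a widget while something overlaps its box.
; Interact opens or closes it according to IsOpen, setting the timeline's play rate from separate open and close durations.
; One timeline plays forward or in reverse to lerp the mesh yaw between closed and open positions.
; IsOpen flips only when the timeline finishes, so interacting mid-swing repeats the current direction.
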(event OnComponentBeginOverlap(Box)
  (params (OverlappedComponent :type Primitive%20Component%20Object%20Reference) (OtherActor :type Actor%20Object%20Reference) (OtherComp :type Primitive%20Component%20Object%20Reference) (OtherBodyIndex :type Integer) (bFromSweep :type Boolean) (SweepResult :type Hit%20Result%20Structure%20%28by%20ref%29))
  (Rendering|SetVisibility (Variables|Default|GetWidget) true false))

(event OnComponentEndOverlap(Box)
  (params (OverlappedComponent :type Primitive%20Component%20Object%20Reference) (OtherActor :type Actor%20Object%20Reference) (OtherComp :type Primitive%20Component%20Object%20Reference) (OtherBodyIndex :type Integer))
  (Rendering|SetVisibility (Variables|Default|GetWidget) false false))

(event Custom|Open%20Door
  (bind _door_track (Timeline|Open%20Door%20T Play)
    (:Update
      (Transformation|SetRelativeRotation (Variables|Default|GetDoor%20StaticMsh) (Math|Rotator|MakeRotator 0.0 0.0 (Math|Float|Lerp (Variables|Default|GetClose%20Position) (Variables|Default|GetOpen%20Position) _door_track)) false false))
    (:Finished
      (Variables|Default|SetIsOpen? (not (Variables|Default|GetIsOpen?))))))

(event Custom|Close%20Door
  (bind _door_track (Timeline|Open%20Door%20T Reverse)
    (:Update
      (Transformation|SetRelativeRotation (Variables|Default|GetDoor%20StaticMsh) (Math|Rotator|MakeRotator 0.0 0.0 (Math|Float|Lerp (Variables|Default|GetClose%20Position) (Variables|Default|GetOpen%20Position) _door_track)) false false))
    (:Finished
      (Variables|Default|SetIsOpen? (not (Variables|Default|GetIsOpen?))))))

(fn ConstructionScript)

(fn Interact
  (params (Interactor :type Character%20Object%20Reference))
  (bind _open_door_t (Variables|Default|GetOpen%20Door%20T))
  (if (not (Variables|Default|GetIsOpen?))
    (Components|Timeline|SetPlayRate _open_door_t (/ 1.0 (Variables|Default|GetTime%20To%20Open%20%28s%29)))
    (CallFunction|OpenDoor)
    (else
      (Components|Timeline|SetPlayRate _open_door_t (/ 1.0 (Variables|Default|GetTime%20To%20Close%20%28s%29)))
      (CallFunction|CloseDoor)))
  (return true))