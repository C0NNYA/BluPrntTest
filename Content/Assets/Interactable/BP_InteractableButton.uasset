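; Interactable button that raises matching makeshift targets, apparently for a shooting range, and shows a widget while something overlaps its sphere.
; An Interact input handler calls UpTarget on every MAkeshift_Target whose TargetValue equals ButtonValue, without checking overlap or CanInteract.
; A second Interact input handler only clears CanInteract and tests DOWN with no effect.
; StartShootingRAnge is empty, and the Interact function just returns true.
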(event OnComponentBeginOverlap(Sphere)
  (params (OverlappedComponent :type Primitive%20Component%20Object%20Reference) (OtherActor :type Actor%20Object%20Reference) (OtherComp :type Primitive%20Component%20Object%20Reference) (OtherBodyIndex :type Integer) (bFromSweep :type Boolean) (SweepResult :type Hit%20Result%20Structure%20%28by%20ref%29))
  (Rendering|SetVisibility (Variables|Default|GetWidget) true false))

(event OnComponentEndOverlap(Sphere)
  (params (OverlappedComponent :type Primitive%20Component%20Object%20Reference) (OtherActor :type Actor%20Object%20Reference) (OtherComp :type Primitive%20Component%20Object%20Reference) (OtherBodyIndex :type Integer))
  (Rendering|SetVisibility (Variables|Default|GetWidget) false false))

(event Custom|StartShootingRAnge)

(event Input|ActionEvents|InputActionInteract
  (params (Key :type Key%20Structure :default "None"))
  (:Pressed
    (if (Variables|Default|GetcanInteract)
      (Variables|Default|SetcanInteract false)
      (if (Variables|Default|GetDOWN?)
        _))))

(event Input|ActionEvents|InputActionInteract
  (params (Key :type Key%20Structure :default "None"))
  (:Pressed
    (bind _outactors (Actor|GetAllActorsOfClass "/Game/Assets/Interactable/MAkeshift_Target.MAkeshift_Target_C"))
    (bind _array_element (Utilities|Array|ForEachLoopwithBreak _outactors)
      (:LoopBody
        (if (== (Variables|/Game/Assets/Interactable/MAkeshift_Target.MAkeshift_Target_C|GetTarget%20value _array_element) (Variables|Default|GetButton%20value))
          (Default|UpTarget _array_element))))))

(fn ConstructionScript)

(fn Interact
  (params (Interactor :type Character%20Object%20Reference))
  (return true))